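; Flying cine camera pawn that is moved by input axes and tuned live like a film camera.
; Mouse yaw and pitch apply only while the look key (<) is held, and R/T variants roll the CineCamera in graded steps.
; Numpad, modifier and mouse-wheel shortcuts set filmback and lens presets, and step focus distance, focal length and aperture.
; The I key toggles a W_CameraInfo widget that receives a reference to this pawn.
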(event Input|AxisEvents|InputAxisMoveForward
  (params (AxisValue :type Float%20%28single-precision%29))
  ;[1 1 1] 1. Camera Movement (With Mouse)
  (Class|DefaultPawn|MoveForward AxisValue))

(event Input|AxisEvents|InputAxisMoveRight
  (params (AxisValue :type Float%20%28single-precision%29))
  ;[1 1 1] 1. Camera Movement (With Mouse)
  (Class|DefaultPawn|MoveRight AxisValue))

(event Input|AxisEvents|InputAxisTurn
  (params (AxisValue :type Float%20%28single-precision%29))
  ;[1 1 1] 1. Camera Movement (With Mouse)
  (if (Variables|Default|GetShiftPressed)
    (Pawn|Input|AddControllerYawInput AxisValue)))

(event Input|AxisEvents|InputAxisLookUp
  (params (AxisValue :type Float%20%28single-precision%29))
  ;[1 1 1] 1. Camera Movement (With Mouse)
  (if (Variables|Default|GetShiftPressed)
    (Pawn|Input|AddControllerPitchInput AxisValue)))

(event Input|AxisEvents|InputAxisMoveUp
  (params (AxisValue :type Float%20%28single-precision%29))
  ;[1 1 1] 1. Camera Movement (With Mouse)
  (Class|DefaultPawn|MoveUpWorld AxisValue))

(event Input|KeyboardEvents|AltSubtract
  (params (Key :type Key%20Structure))
  (bind _cinecamera (Variables|Default|GetCineCamera))
  ;[1 1 1] 5. Aperture
  (:Pressed
    (Variables|/Script/CinematicCamera.CineCameraComponent|SetCurrentAperture _cinecamera (- (Variables|/Script/CinematicCamera.CineCameraComponent|GetCurrentAperture _cinecamera) 0.5))))

(event Input|KeyboardEvents|AltAdd
  (params (Key :type Key%20Structure))
  (bind _cinecamera (Variables|Default|GetCineCamera))
  ;[1 1 1] 5. Aperture
  (:Pressed
    (Variables|/Script/CinematicCamera.CineCameraComponent|SetCurrentAperture _cinecamera (+ (Variables|/Script/CinematicCamera.CineCameraComponent|GetCurrentAperture _cinecamera) 0.5))))

(event Input|MouseEvents|ShiftMouseWheelUp
  (params (Key :type Key%20Structure))
  (bind _cinecamera (Variables|Default|GetCineCamera))
  ;[1 1 1] 6. Focus Distance
  (:Pressed
    (Variables|/Script/CinematicCamera.CineCameraComponent|SetFocusSettings _cinecamera (Utilities|Struct|MakeCameraFocusSettings "Manual" (+ (Variables|/Script/CinematicCamera.CineCameraComponent|GetCurrentFocusDistance _cinecamera) 5e+01)))))

(event Input|MouseEvents|ShiftMouseWheelDown
  (params (Key :type Key%20Structure))
  (bind _cinecamera (Variables|Default|GetCineCamera))
  ;[1 1 1] 6. Focus Distance
  (:Pressed
    (Variables|/Script/CinematicCamera.CineCameraComponent|SetFocusSettings _cinecamera (Utilities|Struct|MakeCameraFocusSettings "Manual" (- (Variables|/Script/CinematicCamera.CineCameraComponent|GetCurrentFocusDistance _cinecamera) 5e+01)))))

(event Input|KeyboardEvents|I
  (params (Key :type Key%20Structure))
  ;[1 1 1] 7. Show/Hide ATH
  (:Pressed
    (Utilities|FlowControl|FlipFlop
      (:A
        (bind _returnvalue (UserInterface|CreateWidget "/Game/Character/CineCam/HUD/W_CameraInfo.W_CameraInfo_C" 0 self))
        (UserInterface|Viewport|AddtoViewport _returnvalue 0))
      (:B
        (Widget|RemovefromParent _returnvalue)))))

(event Input|KeyboardEvents|Subtract
  (params (Key :type Key%20Structure))
  (bind _cinecamera (Variables|Default|GetCineCamera))
  ;[1 1 1] 5. Aperture
  (:Pressed
    (Variables|/Script/CinematicCamera.CineCameraComponent|SetCurrentAperture _cinecamera (- (Variables|/Script/CinematicCamera.CineCameraComponent|GetCurrentAperture _cinecamera) 0.1))))

(event Input|MouseEvents|AltShiftMouseWheelDown
  (params (Key :type Key%20Structure))
  (bind _cinecamera (Variables|Default|GetCineCamera))
  ;[1 1 1] 6. Focus Distance
  (:Pressed
    (Variables|/Script/CinematicCamera.CineCameraComponent|SetFocusSettings _cinecamera (Utilities|Struct|MakeCameraFocusSettings "Manual" (- (Variables|/Script/CinematicCamera.CineCameraComponent|GetCurrentFocusDistance _cinecamera) 1.0)))))

(event Input|KeyboardEvents|<
  (params (Key :type Key%20Structure))
  ;[1 1 1] 1. Camera Movement (With Mouse)
  (:Pressed
    (Variables|Default|SetShiftPressed true))
  (:Released
    (Variables|Default|SetShiftPressed false)))

(event Input|KeyboardEvents|NumPadThree
  (params (Key :type Key%20Structure))
  ;[1 1 1] 2. Filmback Settings
  ;;[1 1 0] Misc (Num 3)
  (:Pressed
    (Variables|/Script/CinematicCamera.CineCameraComponent|SetFilmbackSettings (Variables|Default|GetCineCamera) (Variables|Modes|Others|GetMicro%20Four%20Thirds))))

(event Input|KeyboardEvents|NumPadThree
  (params (Key :type Key%20Structure))
  ;[1 1 1] 2. Filmback Settings
  ;;[1 1 0] Misc (Num 3)
  (:Pressed
    (Variables|/Script/CinematicCamera.CineCameraComponent|SetFilmbackSettings (Variables|Default|GetCineCamera) (Variables|Modes|Others|GetIMAX%2070mm))))

(event Input|KeyboardEvents|CtrlNumPadThree
  (params (Key :type Key%20Structure))
  ;[1 1 1] 2. Filmback Settings
  ;;[1 1 0] Misc (Num 3)
  (:Pressed
    (Variables|/Script/CinematicCamera.CineCameraComponent|SetFilmbackSettings (Variables|Default|GetCineCamera) (Variables|Modes|Others|GetAPS-C%20%28Canon%29))))

(event Input|KeyboardEvents|NumPadZero
  (params (Key :type Key%20Structure))
  ;[1 1 1] 2. Filmback Settings
  ;;[1 0 0] 16:9 (Num 0)
  (:Pressed
    (Variables|/Script/CinematicCamera.CineCameraComponent|SetFilmbackSettings (Variables|Default|GetCineCamera) (Variables|Modes|16:9|Get16:9%20Digital%20Film))))

(event Input|KeyboardEvents|CtrlNumPadZero
  (params (Key :type Key%20Structure))
  ;[1 1 1] 2. Filmback Settings
  ;;[1 0 0] 16:9 (Num 0)
  (:Pressed
    (Variables|/Script/CinematicCamera.CineCameraComponent|SetFilmbackSettings (Variables|Default|GetCineCamera) (Variables|Modes|16:9|Get16:9%20Digital%20Digital%20Film))))

(event Input|KeyboardEvents|CtrlShiftT
  (params (Key :type Key%20Structure))
  (bind _cinecamera (Variables|Default|GetCineCamera))
  (bind _relativerotation (Variables|/Script/Engine.SceneComponent|GetRelativeRotation _cinecamera))
  ;[1 1 1] 7. Rotate (Roll)
  (:Pressed
    (Transformation|SetRelativeRotation _cinecamera (Math|Rotator|MakeRotator (+ (.roll _relativerotation) 1.0) (.pitch _relativerotation) (.yaw _relativerotation)) false false)))

(event Input|KeyboardEvents|AltNumPadZero
  (params (Key :type Key%20Structure))
  ;[1 1 1] 2. Filmback Settings
  ;;[1 0 0] 16:9 (Num 0)
  (:Pressed
    (Variables|/Script/CinematicCamera.CineCameraComponent|SetFilmbackSettings (Variables|Default|GetCineCamera) (Variables|Modes|16:9|Get16:9%20Digital%20DSLR))))

(event Input|KeyboardEvents|NumPadOne
  (params (Key :type Key%20Structure))
  ;[1 1 1] 2. Filmback Settings
  ;;[1 0.5 0] Super XXmm (Num1)
  (:Pressed
    (Variables|/Script/CinematicCamera.CineCameraComponent|SetFilmbackSettings (Variables|Default|GetCineCamera) (Variables|Modes|Super|GetSuper%208mm))))

(event Input|KeyboardEvents|CtrlNumPadOne
  (params (Key :type Key%20Structure))
  ;[1 1 1] 2. Filmback Settings
  ;;[1 0.5 0] Super XXmm (Num1)
  (:Pressed
    (Variables|/Script/CinematicCamera.CineCameraComponent|SetFilmbackSettings (Variables|Default|GetCineCamera) (Variables|Modes|Super|GetSuper%2016mm))))

(event Input|KeyboardEvents|AltNumPadOne
  (params (Key :type Key%20Structure))
  ;[1 1 1] 2. Filmback Settings
  ;;[1 0.5 0] Super XXmm (Num1)
  (:Pressed
    (Variables|/Script/CinematicCamera.CineCameraComponent|SetFilmbackSettings (Variables|Default|GetCineCamera) (Variables|Modes|Super|GetSuper%2035mm))))

(event Input|KeyboardEvents|CtrlNumPadTwo
  (params (Key :type Key%20Structure))
  ;[1 1 1] 2. Filmback Settings
  ;;[1 0.2 0] 35mm (Num2)
  (:Pressed
    (Variables|/Script/CinematicCamera.CineCameraComponent|SetFilmbackSettings (Variables|Default|GetCineCamera) (Variables|Modes|35mm|Get35mm%20Full%20Aperture))))

(event Input|KeyboardEvents|AltNumPadTwo
  (params (Key :type Key%20Structure))
  ;[1 1 1] 2. Filmback Settings
  ;;[1 0.2 0] 35mm (Num2)
  (:Pressed
    (Variables|/Script/CinematicCamera.CineCameraComponent|SetFilmbackSettings (Variables|Default|GetCineCamera) (Variables|Modes|35mm|Get35mm%20VistaVision))))

(event Input|KeyboardEvents|AltNumPadThree
  (params (Key :type Key%20Structure))
  ;[1 1 1] 2. Filmback Settings
  ;;[1 1 0] Misc (Num 3)
  (:Pressed
    (Variables|/Script/CinematicCamera.CineCameraComponent|SetFilmbackSettings (Variables|Default|GetCineCamera) (Variables|Modes|Others|GetFull%20Frame%20DSLR))))

(event Input|KeyboardEvents|CtrlShiftR
  (params (Key :type Key%20Structure))
  (bind _cinecamera (Variables|Default|GetCineCamera))
  (bind _relativerotation (Variables|/Script/Engine.SceneComponent|GetRelativeRotation _cinecamera))
  ;[1 1 1] 7. Rotate (Roll)
  (:Pressed
    (Transformation|SetRelativeRotation _cinecamera (Math|Rotator|MakeRotator (- (.roll _relativerotation) 1.0) (.pitch _relativerotation) (.yaw _relativerotation)) false false)))

(event Input|KeyboardEvents|NumPadTwo
  (params (Key :type Key%20Structure))
  ;[1 1 1] 2. Filmback Settings
  ;;[1 0.2 0] 35mm (Num2)
  (:Pressed
    (Variables|/Script/CinematicCamera.CineCameraComponent|SetFilmbackSettings (Variables|Default|GetCineCamera) (Variables|Modes|35mm|Get35mm%20Academy))))

(event Input|KeyboardEvents|NumPadFour
  (params (Key :type Key%20Structure))
  ;[1 1 1] 3. Lens Settings (Facultatif)
  (:Pressed
    (Variables|/Script/CinematicCamera.CineCameraComponent|SetLensSettings (Variables|Default|GetCineCamera) (Variables|LensSettings|GetUniversal%20Zoom))))

(event Input|KeyboardEvents|T
  (params (Key :type Key%20Structure))
  (bind _cinecamera (Variables|Default|GetCineCamera))
  (bind _relativerotation (Variables|/Script/Engine.SceneComponent|GetRelativeRotation _cinecamera))
  ;[1 1 1] 7. Rotate (Roll)
  (:Pressed
    (Transformation|SetRelativeRotation _cinecamera (Math|Rotator|MakeRotator (+ (.roll _relativerotation) 5.0) (.pitch _relativerotation) (.yaw _relativerotation)) false false)))

(event Input|KeyboardEvents|Add
  (params (Key :type Key%20Structure))
  (bind _cinecamera (Variables|Default|GetCineCamera))
  ;[1 1 1] 5. Aperture
  (:Pressed
    (Variables|/Script/CinematicCamera.CineCameraComponent|SetCurrentAperture _cinecamera (+ (Variables|/Script/CinematicCamera.CineCameraComponent|GetCurrentAperture _cinecamera) 0.1))))

(event Input|KeyboardEvents|CtrlSubtract
  (params (Key :type Key%20Structure))
  ;[1 1 1] 5. Aperture
  (:Pressed
    (Variables|/Script/CinematicCamera.CineCameraComponent|SetCurrentAperture (Variables|Default|GetCineCamera) 2.8)))

(event Input|KeyboardEvents|R
  (params (Key :type Key%20Structure))
  (bind _cinecamera (Variables|Default|GetCineCamera))
  (bind _relativerotation (Variables|/Script/Engine.SceneComponent|GetRelativeRotation _cinecamera))
  ;[1 1 1] 7. Rotate (Roll)
  (:Pressed
    (Transformation|SetRelativeRotation _cinecamera (Math|Rotator|MakeRotator (- (.roll _relativerotation) 5.0) (.pitch _relativerotation) (.yaw _relativerotation)) false false)))

(event Input|KeyboardEvents|CtrlR
  (params (Key :type Key%20Structure))
  (bind _cinecamera (Variables|Default|GetCineCamera))
  (bind _relativerotation (Variables|/Script/Engine.SceneComponent|GetRelativeRotation _cinecamera))
  ;[1 1 1] 7. Rotate (Roll)
  (:Pressed
    (Transformation|SetRelativeRotation _cinecamera (Math|Rotator|MakeRotator (- (.roll _relativerotation) 2.5) (.pitch _relativerotation) (.yaw _relativerotation)) false false)))

(event Input|MouseEvents|CtrlMouseWheelDown
  (params (Key :type Key%20Structure))
  (bind _cinecamera (Variables|Default|GetCineCamera))
  ;[1 1 1] 4. Focal Length
  (:Pressed
    (Variables|/Script/CinematicCamera.CineCameraComponent|SetCurrentFocalLength _cinecamera (- (Variables|/Script/CinematicCamera.CineCameraComponent|GetCurrentFocalLength _cinecamera) 1.0))))

(event Input|MouseEvents|CtrlMouseWheelUp
  (params (Key :type Key%20Structure))
  (bind _cinecamera (Variables|Default|GetCineCamera))
  ;[1 1 1] 4. Focal Length
  (:Pressed
    (Variables|/Script/CinematicCamera.CineCameraComponent|SetCurrentFocalLength _cinecamera (+ (Variables|/Script/CinematicCamera.CineCameraComponent|GetCurrentFocalLength _cinecamera) 1.0))))

(event Input|MouseEvents|AltShiftMouseWheelUp
  (params (Key :type Key%20Structure))
  (bind _cinecamera (Variables|Default|GetCineCamera))
  ;[1 1 1] 6. Focus Distance
  (:Pressed
    (Variables|/Script/CinematicCamera.CineCameraComponent|SetFocusSettings _cinecamera (Utilities|Struct|MakeCameraFocusSettings "Manual" (+ (Variables|/Script/CinematicCamera.CineCameraComponent|GetCurrentFocusDistance _cinecamera) 1.0)))))

(event Input|KeyboardEvents|CtrlT
  (params (Key :type Key%20Structure))
  (bind _cinecamera (Variables|Default|GetCineCamera))
  (bind _relativerotation (Variables|/Script/Engine.SceneComponent|GetRelativeRotation _cinecamera))
  ;[1 1 1] 7. Rotate (Roll)
  (:Pressed
    (Transformation|SetRelativeRotation _cinecamera (Math|Rotator|MakeRotator (+ (.roll _relativerotation) 2.5) (.pitch _relativerotation) (.yaw _relativerotation)) false false)))

(event Input|MouseEvents|CtrlMiddleMouseButton
  (params (Key :type Key%20Structure))
  ;[1 1 1] 4. Focal Length
  (:Pressed
    (Variables|/Script/CinematicCamera.CineCameraComponent|SetCurrentFocalLength (Variables|Default|GetCineCamera) 3e+01)))

(event Input|MouseEvents|AltMouseWheelUp
  (params (Key :type Key%20Structure))
  (bind _cinecamera (Variables|Default|GetCineCamera))
  ;[1 1 1] 6. Focus Distance
  (:Pressed
    (Variables|/Script/CinematicCamera.CineCameraComponent|SetFocusSettings _cinecamera (Utilities|Struct|MakeCameraFocusSettings "Manual" (+ (Variables|/Script/CinematicCamera.CineCameraComponent|GetCurrentFocusDistance _cinecamera) 1e+02)))))

(event Input|MouseEvents|AltMouseWheelDown
  (params (Key :type Key%20Structure))
  (bind _cinecamera (Variables|Default|GetCineCamera))
  ;[1 1 1] 6. Focus Distance
  (:Pressed
    (Variables|/Script/CinematicCamera.CineCameraComponent|SetFocusSettings _cinecamera (Utilities|Struct|MakeCameraFocusSettings "Manual" (- (Variables|/Script/CinematicCamera.CineCameraComponent|GetCurrentFocusDistance _cinecamera) 1e+02)))))

(fn ConstructionScript)